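; Player controller for the Apparatus platformer that turns movement and jump input into detail changes on the controlled subject.
; Each tick, non-zero MoveRight input enables the Walking detail and sets its velocity, while zero input disables it.
; Pressing Jump on a subject with Jumps and OnPlatform details swaps OnPlatform for Jumping, and releasing disables Jumping.
; The controller only toggles ECS-style state and applies no movement itself.
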(event EventTick
  (params (DeltaSeconds :type Float%20%28single-precision%29))
  (bind _returnvalue (Utilities|GetControlledSubject))
  (bind _output_get (Variables|Default|SetGlobalMoveRight (Input|AxisValues|GetMoveRight)))
  (if (!= _output_get 0.0)
    (bind _returnvalue_2 (Class|ApparatusFunctionLibrary|EnableSubjectiveDetail _returnvalue "/Game/ApparatusPlatformer/Details/D_Walking.D_Walking_C"))
    (Variables|/Game/ApparatusPlatformer/Details/D_Walking.D_Walking_C|SetVelocity _returnvalue_2 (Variables|Default|GetGlobalMoveRight))
    (else
      (Class|ApparatusFunctionLibrary|DisableSubjectiveDetail _returnvalue "/Game/ApparatusPlatformer/Details/D_Walking.D_Walking_C" false))))

(event Input|ActionEvents|InputActionJump
  (params (Key :type Key%20Structure :default "None"))
  (bind _returnvalue (Utilities|GetControlledSubject))
  (bind _returnvalue_2 (Utilities|GetControlledSubject))
  (:Pressed
    (if (Class|ApparatusFunctionLibrary|FingerprintMatches (Variables|/Script/ApparatusRuntime.SubjectiveActorComponent|GetFingerprint _returnvalue_2) (|MakeFilter "All" "/Game/ApparatusPlatformer/Details/D_Jumps.D_Jumps_C" "/Game/ApparatusPlatformer/Details/D_OnPlatform.D_OnPlatform_C"))
      (Class|ApparatusFunctionLibrary|DisableSubjectiveDetail _returnvalue "/Game/ApparatusPlatformer/Details/D_OnPlatform.D_OnPlatform_C" false)
      (Class|ApparatusFunctionLibrary|EnableSubjectiveDetail _returnvalue "/Game/ApparatusPlatformer/Details/D_Jumping.D_Jumping_C")))
  (:Released
    (if (Class|ApparatusFunctionLibrary|HasSubjectiveDetail _returnvalue_2 "/Game/ApparatusPlatformer/Details/D_Jumps.D_Jumps_C" false)
      (Class|ApparatusFunctionLibrary|DisableSubjectiveDetail _returnvalue_2 "/Game/ApparatusPlatformer/Details/D_Jumping.D_Jumping_C" false))))

(fn ConstructionScript)